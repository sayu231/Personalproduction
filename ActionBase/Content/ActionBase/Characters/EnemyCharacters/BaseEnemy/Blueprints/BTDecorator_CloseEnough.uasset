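; Behavior tree decorator for enemy AI that decides when movement toward the followed target should end.
; It casts the owner to the AC_EnemyBase controller and measures the distance from its pawn to the TargetToFollow blackboard actor.
; Despite the CloseEnough name, the condition passes while that distance is at least AcceptableDistance and fails once the enemy is closer.
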(fn `PerformConditionCheck`
  (params (OwnerActor :type "Actor Object Reference"))
  (returns (ReturnValue :type Boolean))
  ;[1 1 1] ターゲット方向への移動終了判定
  (bind _asac_enemy_base (cast `/Game/ActionBase/Characters/EnemyCharacters/BaseEnemy/Blueprints/AC_EnemyBase` OwnerActor))
  (set `self.AC_EnemyBase` _asac_enemy_base)
  (return (>= (`KismetMathLibrary.VSize` (- (`Actor.K2_GetActorLocation` (`BTFunctionLibrary.GetBlackboardValueAsActor` (`self.TargetToFollow`))) (`Actor.K2_GetActorLocation` (`Controller.K2_GetPawn` (`self.AC_EnemyBase`))))) (`self.AcceptableDistance`))))