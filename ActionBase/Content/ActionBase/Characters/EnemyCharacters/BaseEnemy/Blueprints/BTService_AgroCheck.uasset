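; Behavior Tree service that handles enemy aggro by detecting visible targets around the AI-controlled pawn.
; Each tick, using the cached AC_EnemyBase controller, it sphere-traces for nearby objects, ignoring all BP_EnemyBase actors.
; A Camera-channel line trace checks sight to each hit, writing visible actors to TargeetToFollow and TargetLocation.
; Blocked or absent hits clear only TargeetToFollow, so the last hit evaluated decides the target.
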(event `self.ReceiveTick`
  (params (OwnerActor :type "Actor Object Reference") (DeltaSeconds :type "Float (single-precision)"))
  (bind _returnvalue (`Actor.K2_GetActorLocation` (`Controller.K2_GetPawn` (`self.AC_EnemyBase`))))
  (if (not (!= (`self.AC_EnemyBase`) null))
    (bind _asac_enemy_base (cast `/Game/ActionBase/Characters/EnemyCharacters/BaseEnemy/Blueprints/AC_EnemyBase` OwnerActor))
    (set `self.AC_EnemyBase` _asac_enemy_base))
  (bind _outactors (`GameplayStatics.GetAllActorsOfClass` "/Game/ActionBase/Characters/EnemyCharacters/BaseEnemy/Blueprints/BP_EnemyBase.BP_EnemyBase_C"))
  (set `self.MyLocation` _returnvalue)
  (bind (_outhits _returnvalue_2) (`KismetSystemLibrary.SphereTraceMultiForObjects` _returnvalue (+ _returnvalue (0.0 0.0 15.0)) 1500.0 (`|MakeArray` (`self.DesiredObjectTypes`)) false _outactors)) ; 敵の探知設定、範囲形状、探知するオブジェクトタイプ
  (if _returnvalue_2
    (for _array_element _outhits
      (bind (_bblockinghit _binitialoverlap _time _distance _location _impactpoint _normal _impactnormal _physmat _hitactor) (`GameplayStatics.BreakHitResult` _array_element))
      (bind _outhit (`KismetSystemLibrary.LineTraceSingle` (`self.MyLocation`) (`Actor.K2_GetActorLocation` _hitactor) "TraceTypeQuery2" false _outactors))
      (bind (_bblockinghit_2 _binitialoverlap_2 _time_2 _distance_2 _location_2 _impactpoint_2 _normal_2 _impactnormal_2 _physmat_2 _hitactor_2) (`GameplayStatics.BreakHitResult` _outhit))
      (if (== _hitactor_2 _hitactor)
        (`BTFunctionLibrary.SetBlackboardValueAsObject` (`self.TargeetToFollow`) _hitactor_2) ; 一致したオブジェクトをBBに渡す
        (`BTFunctionLibrary.SetBlackboardValueAsVector` (`self.TargetLocation`) (`Actor.K2_GetActorLocation` _hitactor_2)) ; 一致したオブジェクトの座標をBBに渡す
        (else
          (`BTFunctionLibrary.SetBlackboardValueAsObject` (`self.TargeetToFollow`)) ; 一致していないからBBに空オブジェクトを渡す
        )))
    (else
      (`BTFunctionLibrary.SetBlackboardValueAsObject` (`self.TargeetToFollow`)))))