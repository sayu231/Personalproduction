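; Base enemy character Blueprint that detects hits from attack collision on its capsule.
; It caches the player at BeginPlay; when a component tagged AttackCollision overlaps, it clears the player's attack collision and damage through an interface message, then calls CallEventHit.
; A separate event stores incoming damage in TakenDamage, but nothing here applies it, as the ApplyDamage node is never executed.
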(event `self.ReceiveBeginPlay`
  (set `self.As_Player` (`GameplayStatics.GetPlayerCharacter` 0)))

(event `self.CapsuleComponent.OnComponentBeginOverlap`
  (params (OverlappedComponent :type "PrimitiveComponent Object Reference") (OtherActor :type "Actor Object Reference") (OtherComp :type "PrimitiveComponent Object Reference") (OtherBodyIndex :type Integer) (bFromSweep :type Boolean) (SweepResult :type "HitResult Structure (by ref)"))
  (`/Engine/EditorBlueprintResources/StandardMacros.IsValid` (`self.As_Player`)
    (:`Is Valid`
      (if (`ActorComponent.ComponentHasTag` OtherComp "AttackCollision")
        (message `/Game/ActionBase/Interface/IF_SetAttackingData.IF_SetAttackingData` (`self.As_Player`) false 0.0) ; 改善の余地あり
        (`self.Event_Hit` false)))))

(event `/Game/ActionBase/Interface/IF_GetAttackDamageDate.GetAttackDamageDate`
  (params (Damage :type "Float (single-precision)"))
  (set `self.Taken_Damage` Damage))

(fn `UserConstructionScript`)